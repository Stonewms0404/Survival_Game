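; Player character Blueprint with axis-driven movement and look, mesh yaw following the camera, and a Health, Stamina and Hunger survival system.
; Looping event timers drain Hunger while Stamina is empty and Health while Hunger is empty, and also clear the stamina-regeneration flag.
; Jumping triggers healing when Health is below its cap, spending Stamina for Health or depleting Hunger when Stamina is short, then prints all three stats.
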(event `InputAxis|Move_Forward/Backwards`
  (params (AxisValue :type "Float (single-precision)"))
  ;[0 0 0 0.502] Movement
  (`self.AddMovementInput` (`KismetMathLibrary.GetForwardVector` (`self.GetControlRotation`)) AxisValue))

(event `InputAxis|Move_Right/Left`
  (params (AxisValue :type "Float (single-precision)"))
  ;[0 0 0 0.502] Movement
  (`self.AddMovementInput` (`KismetMathLibrary.GetRightVector` (`self.GetControlRotation`)) AxisValue))

(event `InputAxis|Look_Up/Down`
  (params (AxisValue :type "Float (single-precision)"))
  ;[0 0 0 0.502] Camera
  (`self.AddControllerPitchInput` AxisValue))

(event `InputAxis|Look_Right/Left`
  (params (AxisValue :type "Float (single-precision)"))
  (bind (_returnvalue_roll _returnvalue_pitch _returnvalue_yaw) (`KismetMathLibrary.BreakRotator` (`self.GetControlRotation`)))
  ;[0 0 0 0.502] Camera
  (`self.AddControllerYawInput` AxisValue)
  (`SceneComponent.K2_SetWorldRotation` (`self.Mesh`) (`KismetMathLibrary.MakeRotator` 0.0 0.0 (+ _returnvalue_yaw -90.0)) false false))

(event `CheckHunger`
  ;[0 0 0 0.5] Hunger Depletion Event
  (if (<= (stale _output_get) 0.0) :!label _label
    (set `self.Hunger` 0.0)
    (set `self.CanRegenerateStamina` false)
    (bind _output_get (set `self.Health` (- (stale _output_get) 1.0)))
    (if (not (`KismetSystemLibrary.K2_IsTimerPausedHandle` (stale _returnvalue)))
      (bind _returnvalue (`KismetSystemLibrary.K2_SetTimerDelegate` (delegate `CheckHunger`) 4.0 true)))
    (else
      (`KismetSystemLibrary.K2_PauseTimerHandle` _returnvalue :!label _label_2))))

(event `DepleteHunger`
  (params (HungerCost :type "Float (double-precision)"))
  ;[0 0 0 0.5] Hunger Depletion Event
  (bind _output_get (set `self.Hunger` (- HungerCost (stale _output_get))))
  (goto _label))

(event `HungerRestored`
  ;[0 0 0 0.5] Hunger Depletion Event
  (set `self.CanRegenerateStamina` true)
  (goto _label_2))

(event `CheckStamina`
  ;[0 0 0 0.5] Stamina Depletion Event
  (if (<= (stale _output_get) 0.0) :!label _label_3
    (set `self.Stamina` 0.0)
    (set `self.CanRegenerateStamina` false)
    (bind _output_get (set `self.Hunger` (- (stale _output_get) 1.0)))
    (if (not true)
      (bind _returnvalue (`KismetSystemLibrary.K2_SetTimerDelegate` (delegate `CheckStamina`) 6.0 true)))
    (else
      (`KismetSystemLibrary.K2_PauseTimerHandle` _returnvalue))))

(event `DepleteStamina`
  (params (StaminaCost :type "Float (double-precision)"))
  ;[0 0 0 0.5] Stamina Depletion Event
  (bind _output_get (set `self.Stamina` (- StaminaCost (stale _output_get))))
  (goto _label_3))

(event `StaminaHealPlayer`
  (bind _health (`self.Health`))
  ;[0 0 0 0.5] Heal Player Via Stamina
  (if (< _health 20.0)
    (if (>= (`self.Stamina`) 2.0)
      (set `self.Health` (+ _health 1.0))
      (`self.DepleteStamina` 2.0)
      (elif (>= (`self.Hunger`) 1.0)
        (`self.DepleteHunger` 1.0)))))

(event `self.OnJumped`
  (`self.StaminaHealPlayer`)
  (`KismetSystemLibrary.PrintString` (`KismetStringLibrary.Concat_StrStr` "Health: " (`KismetStringLibrary.Conv_DoubleToString` (`self.Health`))))
  (`KismetSystemLibrary.PrintString` (`KismetStringLibrary.Concat_StrStr` "Stamina: " (`KismetStringLibrary.Conv_DoubleToString` (`self.Stamina`))))
  (`KismetSystemLibrary.PrintString` (`KismetStringLibrary.Concat_StrStr` "Hunger: " (`KismetStringLibrary.Conv_DoubleToString` (`self.Hunger`)))))

(fn `UserConstructionScript`)